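; BP_Demon is a demon NPC character that shows its Id in an overhead number widget.
; While LookEnemy is enabled, Tick yaws it to face the player, and the setter turns off controller yaw rotation.
; On death it plays a montage, then after a short delay switches to physics ragdoll with movement and capsule collision disabled.
; It also exposes a function to play an alert sound.
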(event `self.ReceiveBeginPlay`
  ;[1 1 1] BeginPlay
  (bind _aswbp_demon_number (cast `/Game/NHG/Characters/NPC/Demon/UI/WBP_DemonNumber` (`WidgetComponent.GetUserWidgetObject` (`self.Widget_HeadNum`)))) ; Character onscreen UI for Id
  (`/Game/NHG/Characters/NPC/Demon/UI/WBP_DemonNumber.SetNumber` _aswbp_demon_number (`self.Id`)))

(event `self.ReceiveTick`
  (params (DeltaSeconds :type "Float (single-precision)"))
  (bind (_returnvalue_roll _returnvalue_pitch _returnvalue_yaw) (`KismetMathLibrary.BreakRotator` (`KismetMathLibrary.ComposeRotators` (`KismetMathLibrary.FindLookAtRotation` (`self.K2_GetActorLocation` (`GameplayStatics.GetPlayerCharacter` 0)) (`self.K2_GetActorLocation`)) (struct :`Yaw` 180.0))))
  ;[1 1 1] Tick
  (if (`self.LookEnemy`)
    (`self.K2_SetActorRotation` (`KismetMathLibrary.MakeRotator` 0.0 0.0 _returnvalue_yaw))))

(event `self.NotifyCharacterDeath`
  ;[1 1 1] On character death
  (`|PlayMontage` (`self.Mesh`) "/Game/AnimStarterPack/Death_3_Montage.Death_3_Montage"
    (:`then`
      (`KismetSystemLibrary.Delay` 0.5)
      (`PrimitiveComponent.SetSimulatePhysics` (`self.Mesh`) true)
      (`ActorComponent.Deactivate` (`self.CharacterMovement`))
      (`PrimitiveComponent.SetCollisionEnabled` (`self.CapsuleComponent`) "NoCollision"))))

(fn `PlayAlertSound`
  (`AudioComponent.Play` (`self.AlertEveryOne_Cue`) 0.0))

(fn `SetEnableLookEnemy`
  (params (Enable :type Boolean))
  (bind _output_get (set `self.LookEnemy` Enable))
  (set `self.bUseControllerRotationYaw` (not _output_get)))

(fn `UserConstructionScript`)