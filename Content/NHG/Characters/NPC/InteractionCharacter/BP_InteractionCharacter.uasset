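; NPC character that coordinates a hand-to-hand interaction point with a TargetCharacter, apparently for hand holding.
; On Tick, the master sets the point at the offset midpoint of both upper-arm sockets and allows interaction within a distance limit.
; Non-masters copy both values from their target through message calls.
; Capsule overlap caches hand locations and plays a timeline, but its lerp never runs, and ending overlap still leaves interaction enabled.
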(event `self.ReceiveTick`
  (params (DeltaSeconds :type "Float (single-precision)"))
  (bind _targetcharacter (`self.TargetCharacter`))
  (if (`self.IsMaster`)
    (bind (_interact _returnvalue) (`self.CalculateInteractionPoint`))
    (set `self.CanInteractTarget` _interact)
    (set `self.TargetCharacterHandLocation` _returnvalue)
    (else
      (bind (_result _location) (message `/Game/NHG/Core/AI/InteractionInterface.GetTargetHandLocation` _targetcharacter))
      (set `self.TargetCharacterHandLocation` _location)
      (bind _interact_2 (message `/Game/NHG/Core/AI/InteractionInterface.CanInteract` _targetcharacter))
      (set `self.CanInteractTarget` _interact_2))))

(event `SetEnableInteraction`
  (params (Enable :type Boolean))
  (`/Engine/EditorBlueprintResources/StandardMacros.IsValid` (`self.TargetCharacter`)
    (:`Is Valid`
      (if Enable
        (bind (_result _location) (message `/Game/NHG/Core/AI/InteractionInterface.GetHandLocation` (`self.TargetCharacter`) (`self.TargetHand`)))
        (if _result
          (set `self.TargetHandLocation` _location)
          (bind (_result_2 _location_2) (`self.GetHandLocation` (`self.InteractionHand`)))
          (if _result_2
            (set `self.CurrentHandLocation` _location_2)
            (`TimelineComponent.Play` (`self.Timeline_HoldHand`))
            (set `self.IsInteractionEnabled` true)))
        (else
          (set `self.IsInteractionEnabled` true))))))

(event `self.CapsuleComponent.OnComponentBeginOverlap`
  (params (OverlappedComponent :type "PrimitiveComponent Object Reference") (OtherActor :type "Actor Object Reference") (OtherComp :type "PrimitiveComponent Object Reference") (OtherBodyIndex :type Integer) (bFromSweep :type Boolean) (SweepResult :type "HitResult Structure (by ref)"))
  (if (== OtherActor (`self.TargetCharacter`))
    (`self.SetEnableInteraction` true)))

(event `self.CapsuleComponent.OnComponentEndOverlap`
  (params (OverlappedComponent :type "PrimitiveComponent Object Reference") (OtherActor :type "Actor Object Reference") (OtherComp :type "PrimitiveComponent Object Reference") (OtherBodyIndex :type Integer))
  (if (== OtherActor (`self.TargetCharacter`))
    (`self.SetEnableInteraction` false)))

(fn `CalculateInteractionPoint`
  (returns (Interact :type Boolean) (ReturnValue :type "Vector Structure"))
  (locals (UpperArmLocation :type "Vector Structure" :default (0.0 0.0 0.0)) (TargetUpperArmLocation :type "Vector Structure" :default (0.0 0.0 0.0)))
  (`/Engine/EditorBlueprintResources/StandardMacros.IsValid` (`self.TargetCharacter`)
    (:`Is Valid`
      (set `local.UpperArmLocation` (`SceneComponent.GetSocketLocation` (`self.Mesh`) (select `/Game/NHG/Characters/NPC/InteractionCharacter/EInteractionHand` (`self.InteractionHand`) :`NewEnumerator1` "upperarm_l" :`NewEnumerator2` "upperarm_r" :!type "Name")))
      (set `local.TargetUpperArmLocation` (`SceneComponent.GetSocketLocation` (`Character.Mesh` (`self.TargetCharacter`)) (select `/Game/NHG/Characters/NPC/InteractionCharacter/EInteractionHand` (`self.TargetHand`) :`NewEnumerator1` "upperarm_l" :`NewEnumerator2` "upperarm_r" :!type "Name")))
      (bind _returnvalue (`self.GetMidPoint` (`local.UpperArmLocation`) (`local.TargetUpperArmLocation`)))
      (return (<= (`KismetMathLibrary.Vector_Distance` (`local.UpperArmLocation`) (`local.TargetUpperArmLocation`)) (`self.MasterInteractionDistance`)) (+ _returnvalue (`self.InteractionOffset`))))))

(fn `CanInteract`
  (returns (Interact :type Boolean))
  (return (`self.CanInteractTarget`)))

(fn `GetCurrentInteractionHand`
  (returns (Hand :type "/Game/NHG/Characters/NPC/InteractionCharacter/EInteractionHand Enum"))
  (return (`self.InteractionHand`)))

(fn `GetHandLocation`
  (params (Hand :type "/Game/NHG/Characters/NPC/InteractionCharacter/EInteractionHand Enum" :default "NewEnumerator0"))
  (returns (Result :type Boolean) (Location :type "Vector Structure"))
  (if (`|EnumInequality` Hand "NewEnumerator0")
    (return true (`SceneComponent.GetSocketLocation` (`self.Mesh`) (select `/Game/NHG/Characters/NPC/InteractionCharacter/EInteractionHand` (`self.InteractionHand`) :`NewEnumerator1` "hand_l" :`NewEnumerator2` "hand_r" :!type "Name")))
    (else
      (return false (0.0 0.0 0.0)))))

(fn `GetMidPoint`
  (params (V1 :type "Vector Structure") (V2 :type "Vector Structure"))
  (returns (ReturnValue :type "Vector Structure"))
  (return (/ (+ V1 V2) 2.0)))

(fn `GetTargetHandLocation`
  (returns (Result :type Boolean) (Location :type "Vector Structure"))
  (return true (`self.TargetCharacterHandLocation`)))

(fn `UserConstructionScript`)