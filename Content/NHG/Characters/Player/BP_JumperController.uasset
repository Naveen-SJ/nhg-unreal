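; BP_JumperController is a player controller that makes the controlled BP_Jumper jump to the point clicked on the map.
; On left click it traces from the cursor into the world and offsets the hit by the capsule height.
; It computes a launch velocity from pawn location, gravity and jump height, then passes it to CustomJump.
; A WBP_JumperControls widget, created at BeginPlay, supplies the multiplier that scales MaxJumpHeight.
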(event `self.ReceiveBeginPlay`
  (`|ExecutionSequence`
    (:`then_0`
      (bind _returnvalue (`|CreateWidget` "/Game/NHG/Widgets/WBP_JumperControls.WBP_JumperControls_C"))
      (`UserWidget.AddToViewport` _returnvalue 0)
      (set `self.Multiplier` (`/Game/NHG/Widgets/WBP_JumperControls.GetCurrentMultiplierValue` _returnvalue))
      (add `/Game/NHG/Widgets/WBP_JumperControls.OnHeightMultiplierChanged` _returnvalue (`|CreateDelegate` :!event `OnHeightMultiplierChanged`)))
    (:`then_1`
      (set `self.bShowMouseCursor` true))))

(event `OnHeightMultiplierChanged`
  (params (Multipier :type "Float (double-precision)"))
  (set `self.Multiplier` Multipier))

(event `Key|LeftMouseButton`
  (params (Key :type "Key Structure"))
  (bind (_locationx _locationy) (`self.GetMousePosition`))
  (bind (_worldposition _worlddirection _returnvalue) (`GameplayStatics.DeprojectScreenToWorld` self (`KismetMathLibrary.MakeVector2D` _locationx _locationy)))
  (:`Pressed`
    (if _returnvalue
      (bind (_outhit _returnvalue_2) (`KismetSystemLibrary.LineTraceSingle` _worldposition (+ _worldposition (* _worlddirection 500000.0)) "TraceTypeQuery1")) ; Try get mouse click location on map
      (if _returnvalue_2
        (bind _output_get (set `self.TargetLocation` (+ (`.Location` (`GameplayStatics.BreakHitResult` _outhit)) (0.0 0.0 88.0))))
        (bind _velocity (`BPFunctionLibrary.CalculateLaunchVelocity` (`self.GetStartLocation`) _output_get (`self.GetJumpHeight`) (`self.GetGravity`)))
        (bind _asbp_jumper (cast `/Game/NHG/Characters/Player/BP_Jumper` (`self.K2_GetPawn`)))
        (`/Game/NHG/Characters/Player/BP_Jumper.CustomJump` _asbp_jumper _velocity (`self.TargetLocation`))))))

(fn `GetGravity`
  (returns (ReturnValue :type "Float (double-precision)"))
  (bind _ascharacter (cast `Character` (`self.K2_GetPawn`))
    (:`then`
      (return (`MovementComponent.GetGravityZ` (`Character.CharacterMovement` _ascharacter))))
    (:`CastFailed`
      (return 0.0))))

(fn `GetJumpHeight`
  (returns (ReturnValue :type "Float (double-precision)"))
  (return (* (`self.MaxJumpHeight`) (`self.Multiplier`))))

(fn `GetStartLocation`
  (returns (ReturnValue :type "Vector Structure"))
  (return (`self.K2_GetActorLocation` (`self.K2_GetPawn`))))

(fn `UserConstructionScript`)