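; BP_NhgGameInstance is the game instance, providing a SetEnablePause event that toggles game pause together with the map menu.
; Pausing creates a new WBP_MapMenu, adds it to the viewport at Z-order 10, caches the player controller's cursor visibility and shows the cursor.
; Unpausing removes the stored widget and restores the cached cursor state, provided the widget is valid.
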(event `/Game/NHG/Core/GamePlay/GamePauseInterface.SetEnablePause`
  (params (Enable :type Boolean))
  (bind _returnvalue (`GameplayStatics.GetPlayerController` 0))
  (bind _mapmenuwidget (`self.MapMenuWidget`))
  (`GameplayStatics.SetGamePaused` Enable)
  (if Enable
    (bind _returnvalue_2 (`|CreateWidget` "/Game/NHG/Widgets/WBP_MapMenu.WBP_MapMenu_C"))
    (bind _output_get (set `self.MapMenuWidget` _returnvalue_2))
    (`UserWidget.AddToViewport` _output_get 10)
    (set `self.MouseCursor` (`PlayerController.bShowMouseCursor` _returnvalue))
    (set `PlayerController.bShowMouseCursor` true _returnvalue)
    (else
      (`/Engine/EditorBlueprintResources/StandardMacros.IsValid` _mapmenuwidget
        (:`Is Valid`
          (`Widget.RemoveFromParent` _mapmenuwidget)
          (set `PlayerController.bShowMouseCursor` (`self.MouseCursor`) (`GameplayStatics.GetPlayerController` 0)))))))