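; BP_CombatManager limits which AI controllers engage in combat at once, favoring those closest to their enemy.
; A looping one-second timer picks the nearest registered controller failing CanEngageInCombat and tries to engage it, displacing the farthest engaged AI if refused and closer.
; Registration attempts engagement immediately, while unregistration reruns the token update.
; Tick draws debug lines from engaged AI to the player, marked for removal in final builds.
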(event `self.ReceiveBeginPlay`
  ;[1 1 1] BeginPlay
  (bind _returnvalue (`KismetSystemLibrary.K2_SetTimerDelegate` (`|CreateDelegate` :!event `TokenUpdate`) 1.0 true))
  (set `self.TokenUpdateTimer` _returnvalue))

(event `TokenUpdate`
  ;[1 1 1] TokenUpdate
  (bind (_result _controller) (`self.GetClosetCharacterToEngage`))
  (if _result
    (bind _returnvalue (`self.AddControllerToEngageInCombat` _controller))
    (if (not _returnvalue)
      (bind (_result_2 _controller_2) (`self.GetFarestEngagedCharacter`))
      (if _result_2
        (if (> (`AIControllerBase.GetDistanceFromEnemy` _controller_2) (`AIControllerBase.GetDistanceFromEnemy` _controller))
          (`self.RemoveControllerFromCombat` _controller_2)
          (`self.AddControllerToEngageInCombat` _controller))
        (else
          (`self.AddControllerToEngageInCombat` _controller))))))

(event `self.ReceiveTick`
  (params (DeltaSeconds :type "Float (single-precision)"))
  ;[1 1 1] Tick
  (`|ExecutionSequence`
    (:`then_0`
      (for _array_element (`self.EngagedAI`)
        (`KismetSystemLibrary.DrawDebugLine` (`self.K2_GetActorLocation` (`AIControllerBase.GetControllerAICharacter` _array_element)) (`self.K2_GetActorLocation` (`GameplayStatics.GetPlayerCharacter` 0)) (struct :`R` 0.053955 :`G` 0.084747 :`B` 0.609375 :`A` 1.0) 0.0 5.0)))))

(event `self.NotifyOnControllerRegistered`
  (params (ControllerBase :type "AIControllerBase Object Reference") (Enemy :type "CharacterBase Object Reference"))
  ;[1 1 1] On AI controller registered for combat
  (`self.AddControllerToEngageInCombat` ControllerBase))

(event `self.NotifyOnControllerUnregistered`
  (params (ControllerBase :type "AIControllerBase Object Reference"))
  ;[1 1 1] On AI controller unregisters from combat
  (`self.TokenUpdate`))

(fn `GetClosetCharacterToEngage`
  (returns (Result :type Boolean) (Controller :type "AIControllerBase Object Reference"))
  (locals (MinDistance :type "Float (double-precision)") (SelectedController :type "AIControllerBase Object Reference"))
  (bind _selectedcontroller (`local.SelectedController`))
  (set `local.MinDistance` 10000000.0)
  (for _array_element (`self.RegisteredAIControllerList`)
    (if (not (`AIControllerBase.CanEngageInCombat` _array_element))
      (bind _returnvalue (`AIControllerBase.GetDistanceFromEnemy` _array_element))
      (if (> (`local.MinDistance`) _returnvalue)
        (set `local.SelectedController` _array_element)
        (set `local.MinDistance` _returnvalue))))
  (`/Engine/EditorBlueprintResources/StandardMacros.IsValid` _selectedcontroller
    (:`Is Valid`
      (return true _selectedcontroller))
    (:`Is Not Valid`
      (return false null))))

(fn `GetFarestEngagedCharacter`
  (returns (Result :type Boolean) (Controller :type "AIControllerBase Object Reference"))
  (locals (MaxDistance :type "Float (double-precision)") (SelectedController :type "AIControllerBase Object Reference"))
  (bind _selectedcontroller (`local.SelectedController`))
  (set `local.MaxDistance` 0.0)
  (for _array_element (`self.EngagedAI`)
    (bind _returnvalue (`KismetMathLibrary.Vector_Distance` (`self.K2_GetActorLocation` (`AIControllerBase.GetControllerAICharacter` _array_element)) (`self.K2_GetActorLocation` (`AIControllerBase.GetEnemyCharacter` _array_element))))
    (if (> _returnvalue (`local.MaxDistance`))
      (set `local.SelectedController` _array_element)
      (set `local.MaxDistance` _returnvalue)))
  (`/Engine/EditorBlueprintResources/StandardMacros.IsValid` _selectedcontroller
    (:`Is Valid`
      (return true _selectedcontroller))
    (:`Is Not Valid`
      (return false null))))

(fn `UserConstructionScript`)